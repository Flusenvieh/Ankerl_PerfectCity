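; GA_SimpleShot is a Gameplay Ability that fires a hitscan shot for the player character.
; After committing, it line traces from the third-person camera, then from the mouth socket to that impact point, drawing debug lines for both.
; An actor hit by the second trace receives the GE_SimpleShot_Damage effect if it has an Ability System Component.
; A failed commit tries to activate the Reload ability by tag before ending.
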(event Ability|EventActivateAbility
  (bind _returnvalue (Ability|GetAbilitySystemComponentfromActorInfo))
  (bind _draw_time (Variables|Default|GetDraw%20Time))
  (bind _asbp_player_character (Utilities|Casting|CastToBP_PlayerCharacter (Ability|GetAvatarActorfromActorInfo)))
  (Variables|Default|SetPlayer%20Character _asbp_player_character)
  (bind _returnvalue_2 (Ability|CommitAbility))
  (if _returnvalue_2
    (Utilities|FlowControl|Sequence
      (:then_0
        (bind (_outhit _returnvalue_3) (Collision|LineTraceByChannel (Transformation|GetWorldLocation (Variables|/Script/PerfectCity.PCPlayerCharacter|GetThirdPersonCameraComponent (Variables|Default|GetPlayer%20Character))) (+ (Transformation|GetWorldLocation (Variables|/Script/PerfectCity.PCPlayerCharacter|GetThirdPersonCameraComponent (Variables|Default|GetPlayer%20Character))) (* (Math|Vector|GetForwardVector (Variables|/Script/PerfectCity.PCPlayerCharacter|GetThirdPersonCameraComponent (Variables|Default|GetPlayer%20Character))) (Variables|Default|GetRange))) "TraceTypeQuery2" false 0 "ForDuration" true "(R=0.447917,G=0.000000,B=0.000000,A=1.000000)" "(R=0.000000,G=0.307292,B=0.000000,A=1.000000)" _draw_time)) ; First trace from camera
        (if _returnvalue_3
          (bind _outhit_2 (Collision|LineTraceByChannel (Transformation|GetSocketLocation (Class|GameplayAbility|GetOwningComponentfromActorInfo) "socket_mouth") (.ImpactPoint (Collision|BreakHitResult _outhit)) "TraceTypeQuery2" false 0 "ForDuration" true "(R=1.000000,G=0.000000,B=0.000000,A=1.000000)" "(R=0.000000,G=1.000000,B=0.000000,A=1.000000)" _draw_time)) ; Then trace from Socket
          (Utilities|IsValid (Ability|GetAbilitySystemComponent (.HitActor (Collision|BreakHitResult _outhit_2)))
            (:Is%20Valid
              (GameplayEffects|ApplyGameplayEffectSpecToTarget _returnvalue (Ability|MakeOutgoingGameplayEffectSpec "/Game/Player/Abilities/GE_SimpleShot_Damage.GE_SimpleShot_Damage_C") (Ability|GetAbilitySystemComponent (.HitActor (Collision|BreakHitResult _outhit_2))))))))
      (:then_1
        (Ability|EndAbility :!label _label)))
    (else
      (Abilities|TryActivateAbilitiesbyTag _returnvalue (GameplayTags|MakeGameplayTagContainerfromTag "(TagName=\"Ability.Type.Active.Reload\")") true)
      (goto _label))))

(event Ability|EventOnEndAbility
  (params (bWasCancelled :type Boolean)))