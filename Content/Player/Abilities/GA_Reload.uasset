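; GA_Reload is a player gameplay ability that instantly reloads ammo.
; On activation it commits, checks that an attribute lookup succeeded, and computes the difference between two float attribute reads, presumably maximum and current ammo.
; That difference feeds the GE_Reload_SetByCaller effect as a SetByCaller magnitude tagged Resource.Ammo.Current, applied to the owner's ability system.
; The ability then ends, as it also does when the commit or lookup fails.
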(event Ability|EventActivateAbility
  (bind _returnvalue (Ability|GetAbilitySystemComponentfromActorInfo))
  (bind (_bsuccessfullyfoundattribute _returnvalue_2) (Ability|Attribute|GetFloatAttributefromAbilitySystemComponent _returnvalue "(AttributeName=\"MaxAmmo\",Attribute=/Script/PerfectCity.PCCombatAttributeSet:MaxAmmo,AttributeOwner=\"/Script/CoreUObject.Class'/Script/PerfectCity.PCCombatAttributeSet'\")"))
  (bind _returnvalue_3 (Ability|CommitAbility))
  (if (and _returnvalue_3 _bsuccessfullyfoundattribute)
    (Utilities|FlowControl|Sequence
      (:then_0
        (bind _returnvalue_4 (Ability|GameplayEffect|AssignTagSetbyCallerMagnitude (GameplayEffects|MakeOutgoingSpec :self _returnvalue :GameplayEffectClass "/Game/Player/Abilities/GE_Reload_SetByCaller.GE_Reload_SetByCaller_C") "(TagName=\"Resource.Ammo.Current\")" (- _returnvalue_2 (.ReturnValue (Ability|Attribute|GetFloatAttributefromAbilitySystemComponent _returnvalue "(AttributeName=\"Ammo\",Attribute=/Script/PerfectCity.PCCombatAttributeSet:Ammo,AttributeOwner=\"/Script/CoreUObject.Class'/Script/PerfectCity.PCCombatAttributeSet'\")")))))
        (GameplayEffects|ApplyGameplayEffectSpecToSelf _returnvalue _returnvalue_4))
      (:then_1
        (Ability|EndAbility :!label _label)))
    (else
      (goto _label))))

(event Ability|EventOnEndAbility
  (params (bWasCancelled :type Boolean)))