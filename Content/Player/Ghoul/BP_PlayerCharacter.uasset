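; Player character Blueprint that creates and updates the local player's HUD for health and ammo.
; On BeginPlay, a locally controlled instance creates the WI_HUD widget and seeds its health and ammo from Ability System Component attributes.
; Health and ammo change events then push new values to that widget, again only when locally controlled, with ammo truncated to whole numbers.
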(event EventBeginPlay
  (bind _abilitysystemcomponent (Variables|Default|GetAbilitySystemComponent))
  (if (Pawn|IsLocallyControlled)
    (bind _returnvalue (UserInterface|CreateWidget "/Game/UI/WI_HUD.WI_HUD_C"))
    (Variables|Default|SetHud _returnvalue)
    (UserInterface|Viewport|AddtoViewport _returnvalue 0)
    (Default|Init (Variables|/Game/UI/WI_HUD.WI_HUD_C|GetWI_Health _returnvalue) (.ReturnValue (Class|AbilitySystemComponent|GetGameplayAttributeValue _abilitysystemcomponent "(AttributeName=\"MaxHealth\",Attribute=/Script/PerfectCity.PCHealthAttributeSet:MaxHealth,AttributeOwner=\"/Script/CoreUObject.Class'/Script/PerfectCity.PCHealthAttributeSet'\")")) (.ReturnValue (Class|AbilitySystemComponent|GetGameplayAttributeValue _abilitysystemcomponent "(AttributeName=\"Health\",Attribute=/Script/PerfectCity.PCHealthAttributeSet:Health,AttributeOwner=\"/Script/CoreUObject.Class'/Script/PerfectCity.PCHealthAttributeSet'\")")))
    (Variables|/Game/UI/WI_HUD.WI_HUD_C|SetAmmo _returnvalue (Math|Float|Truncate (.ReturnValue (Ability|Attribute|GetFloatAttributefromAbilitySystemComponent _abilitysystemcomponent "(AttributeName=\"Ammo\",Attribute=/Script/PerfectCity.PCCombatAttributeSet:Ammo,AttributeOwner=\"/Script/CoreUObject.Class'/Script/PerfectCity.PCCombatAttributeSet'\")"))))))

(event Collision|EventActorBeginOverlap
  (params (OtherActor :type Actor%20Object%20Reference)))

(event EventTick
  (params (DeltaSeconds :type Float%20%28single-precision%29)))

(event EventOnHealthChanged
  (params (OldValue :type Float%20%28single-precision%29) (NewValue :type Float%20%28single-precision%29))
  (if (Pawn|IsLocallyControlled)
    (Default|SetCurrentHealth (Variables|/Game/UI/WI_HUD.WI_HUD_C|GetWI_Health (Variables|Default|GetHud)) NewValue)))

(event EventOnAmmoChanged
  (params (OldValue :type Float%20%28single-precision%29) (NewValue :type Float%20%28single-precision%29))
  (if (Pawn|IsLocallyControlled)
    (Variables|/Game/UI/WI_HUD.WI_HUD_C|SetAmmo (Variables|Default|GetHud) (Math|Float|Truncate NewValue))))

(fn ConstructionScript)