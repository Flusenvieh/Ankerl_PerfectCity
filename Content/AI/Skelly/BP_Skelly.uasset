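; BP_Skelly is the Skelly AI pawn, which reacts to taking damage and dying.
; HandleHealthChanged acts only when health drops and the pawn is locally controlled.
; If health remains, it writes the damage causer to the AI controller's Blackboard as EnemyActor and sets HasLineOfSight true, without a sight check.
; Otherwise it destroys itself immediately; the construction script and other events are empty.
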(event EventBeginPlay)

(event Collision|EventActorBeginOverlap
  (params (OtherActor :type Actor%20Object%20Reference)))

(event EventTick
  (params (DeltaSeconds :type Float%20%28single-precision%29)))

(event EventHandleHealthChanged
  (params (DamageInstigator :type Actor%20Object%20Reference) (DamageCauser :type Actor%20Object%20Reference) (DamageMagnitude :type Float%20%28single-precision%29) (OldValue :type Float%20%28single-precision%29) (NewValue :type Float%20%28single-precision%29))
  (bind _self self)
  (bind _returnvalue (AI|GetAIController _self))
  (bind _blackboard (Variables|/Script/AIModule.AIController|GetBlackboard _returnvalue))
  (if (and (Pawn|IsLocallyControlled) (> OldValue NewValue))
    (if (> NewValue 0.0)
      (AI|Components|Blackboard|SetValueasObject _blackboard (Variables|Default|GetEnemyActor) DamageCauser)
      (AI|Components|Blackboard|SetValueasBool _blackboard (Variables|Default|GetHasLineOfSight) true)
      (else
        (Actor|DestroyActor)))))

(fn ConstructionScript)